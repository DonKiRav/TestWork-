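; BP_TargetActor is a target actor that carries a Widget component displaying its identity info.
; On BeginPlay it copies its Sprite, Gender, Name and Index variables into the WBP_Statistic widget, converting the gender enum to text.
; FunctionShowInfo and FunctionCloseInfo events toggle that component's visibility; no caller for them appears within this Blueprint.
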(event `/Game/TargetActors/Interface/BPI_TargetActorInterface.Function_CloseInfo`
  (`SceneComponent.SetVisibility` (`self.Widget`) false false))

(event `/Game/TargetActors/Interface/BPI_TargetActorInterface.Function_ShowInfo`
  (`SceneComponent.SetVisibility` (`self.Widget`) true false))

(event `self.ReceiveBeginPlay`
  (`self.Function_SetInfoToWidget`))

(fn `Function_SetInfoToWidget`
  (bind _aswbp_statistic (cast `/Game/TargetActors/UI/WBP_Statistic` (`WidgetComponent.GetWidget` (`self.Widget`))))
  (`Image.SetBrushFromTexture` (`/Game/TargetActors/UI/WBP_Statistic.Sprite` _aswbp_statistic) (`self.sprite`) false)
  (`TextBlock.SetText` (`/Game/TargetActors/UI/WBP_Statistic.Text_Gender` _aswbp_statistic) (`KismetTextLibrary.Conv_StringToText` (`|GetEnumeratorNameAsString` (`self.gender`))))
  (`TextBlock.SetText` (`/Game/TargetActors/UI/WBP_Statistic.Text_Name` _aswbp_statistic) (`KismetTextLibrary.Conv_StringToText` (`self.name`)))
  (`TextBlock.SetText` (`/Game/TargetActors/UI/WBP_Statistic.Text_Index` _aswbp_statistic) (`KismetTextLibrary.Conv_IntToText` (`self.index`))))

(fn `UserConstructionScript`)